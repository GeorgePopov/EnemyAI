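; Character component that runs bow combat: it equips a bow on BeginPlay and handles aiming, drawing and firing arrows.
; Aiming switches the owner to controller-facing rotation and spawns a socketed arrow.
; Drawing builds DrawTime on a looping timer; firing launches the arrow along camera forward at normalized draw strength, then re-aims after the montage.
; Gameplay tags gate each stage, and the bow's state follows along.
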(event `self.ReceiveBeginPlay`
  (bind _ascharacter (cast `Character` (`self.GetOwner`)))
  (bind _output_get (set `self.AsOwner` _ascharacter))
  (`self.EquipBow`)
  (set `self.GameplayTags` (`Actor.GetComponentByClass` _output_get "/Game/Framework/GameplayTags/AC_GameplayTags.AC_GameplayTags_C")))

(event `AimBegin`
  (bind _charactermovement (`Character.CharacterMovement` (`self.AsOwner`)))
  ; Aim Bow
  (message `/Game/Framework/GameplayTags/BPI_GameplayTagFunction.AddGameplayTags` (`self.GameplayTags`) (struct :`GameplayTags` (struct :`(TagName` "Character.IsAiming"))))
  (set `CharacterMovementComponent.bOrientRotationToMovement` false _charactermovement)
  (set `CharacterMovementComponent.bUseControllerDesiredRotation` true _charactermovement)
  (set `CharacterMovementComponent.RotationRate` (struct :`Yaw` 1000.0) _charactermovement)
  (set `/Game/Framework/Weapons/BP_Bow.BowState` "NewEnumerator1" (`self.Bow`))
  (`self.SpawnArrow`))

(event `AimEnd`
  (bind _charactermovement (`Character.CharacterMovement` (`self.AsOwner`)))
  ; Aim Bow
  (`self.DrawEnd`)
  (message `/Game/Framework/GameplayTags/BPI_GameplayTagFunction.RemoveGameplayTags` (`self.GameplayTags`) (struct :`GameplayTags` (struct :`(TagName` "Character.IsAiming"))))
  (set `CharacterMovementComponent.bOrientRotationToMovement` true _charactermovement)
  (set `CharacterMovementComponent.bUseControllerDesiredRotation` false _charactermovement)
  (set `CharacterMovementComponent.RotationRate` (struct :`Yaw` 500.0) _charactermovement)
  (set `/Game/Framework/Weapons/BP_Bow.BowState` "NewEnumerator0" (`self.Bow`))
  (`self.DestroyArrow`))

(event `DrawBegin`
  (bind _gameplaytags (`self.GameplayTags`))
  ; Draw Bow
  (bind _returnvalue (message `/Game/Framework/GameplayTags/BPI_GameplayTagFunction.HasActiveGameplayTag` _gameplaytags (struct :`TagName` "Character.IsDrawingBow") true))
  (bind _returnvalue_2 (message `/Game/Framework/GameplayTags/BPI_GameplayTagFunction.HasActiveGameplayTag` _gameplaytags (struct :`TagName` "Character.IsAiming") true))
  (if (and _returnvalue_2 (not _returnvalue) (not (`self.IsFiringArrow`)))
    (message `/Game/Framework/GameplayTags/BPI_GameplayTagFunction.AddGameplayTags` (`self.GameplayTags`) (struct :`GameplayTags` (struct :`(TagName` "Character.IsDrawingBow"))))
    (bind _returnvalue_3 (`KismetSystemLibrary.K2_SetTimerDelegate` (delegate `IncrementDrawTime`) (`self.DrawIncrementTime`) true))
    (set `self.DrawBowTimer` _returnvalue_3)
    (set `/Game/Framework/Weapons/BP_Bow.BowState` "NewEnumerator2" (`self.Bow`))))

(event `IncrementDrawTime`
  ; Draw Bow
  (set `self.DrawTime` (+ (`self.DrawTime`) (`self.DrawIncrementTime`))))

(event `DrawEnd`
  ; Draw Bow
  (set `self.DrawTime` 0.0)
  (message `/Game/Framework/GameplayTags/BPI_GameplayTagFunction.RemoveGameplayTags` (`self.GameplayTags`) (struct :`GameplayTags` (struct :`(TagName` "Character.IsDrawingBow"))))
  (`KismetSystemLibrary.K2_ClearAndInvalidateTimerHandle` (`self.DrawBowTimer`))
  (set `/Game/Framework/Weapons/BP_Bow.BowState` "NewEnumerator0" (`self.Bow`)))

(event `FireArrowBegin`
  ; Fire Arrow
  (bind _returnvalue (message `/Game/Framework/GameplayTags/BPI_GameplayTagFunction.HasActiveGameplayTag` (`self.GameplayTags`) (struct :`TagName` "Character.IsDrawingBow") true))
  (if _returnvalue
    (set `self.IsFiringArrow` true)
    (`self.FireArrow`)
    (`self.DrawEnd`)
    (`|PlayMontage` (`Character.Mesh` (`self.AsOwner`)) (`self.Fire_Montage`)
      (:`OnCompleted`
        _)
      (:`OnInterrupted`
        _))
    (`self.FireArrowEnd`)))

(event `FireArrowEnd`
  ; Fire Arrow
  (set `self.IsFiringArrow` false)
  (bind _returnvalue (message `/Game/Framework/GameplayTags/BPI_GameplayTagFunction.HasActiveGameplayTag` (`self.GameplayTags`) (struct :`TagName` "Character.IsAiming") true))
  (if _returnvalue
    (`self.AimBegin`)))

(fn `DestroyArrow`
  (bind _arrow (`self.Arrow`)
    (:`then`
      (`Actor.K2_DestroyActor` _arrow)
      (return))
    (:`else`)))

(fn `EquipBow`
  (bind _returnvalue (`|SpawnActorFromClass` "/Game/Framework/Weapons/BP_Bow.BP_Bow_C" (`KismetMathLibrary.MakeTransform` (0.0 0.0 0.0)) "Undefined" "MultiplyWithRoot" null null)) ; Если сюда нужно передать разные луки для экипировки,\nиз Class делаем переменную и сетим её в персонаже.\nТогда проблемы с постоянной переменной, узнать у гемини
  (bind _output_get (set `self.Bow` _returnvalue))
  (`Actor.K2_AttachToComponent` _output_get (`Character.Mesh` (`self.AsOwner`)) (`self.Bow_SocketName`) "SnapToTarget" "SnapToTarget" "SnapToTarget" true)
  (return))

(fn `FireArrow`
  (bind _arrow (`self.Arrow`)
    (:`then`
      (`Actor.K2_DetachFromActor` _arrow "KeepWorld" "KeepWorld" "KeepWorld")
      (`/Game/Framework/Weapons/BP_Arrow.Fire` _arrow (`SceneComponent.GetForwardVector` (`Actor.GetComponentByClass` (`self.AsOwner`) "/Script/Engine.CameraComponent")) (`KismetMathLibrary.FClamp` (`KismetMathLibrary.NormalizeToRange` (`self.DrawTime`) 0.0 (`/Game/Framework/Weapons/BP_Bow.MaxDrawTime` (`self.Bow`)))))
      (set `self.Arrow` null)
      (return))
    (:`else`)))

(fn `SpawnArrow`
  (bind _returnvalue (`|SpawnActorFromClass` "/Game/Framework/Weapons/BP_Arrow.BP_Arrow_C" (`KismetMathLibrary.MakeTransform` (0.0 0.0 0.0)) "Undefined" "MultiplyWithRoot" null null))
  (bind _output_get (set `self.Arrow` _returnvalue))
  (`Actor.K2_AttachToComponent` _output_get (`Character.Mesh` (`self.AsOwner`)) (`self.Arrow_SocketName`) "SnapToTarget" "SnapToTarget" "SnapToTarget" true)
  (return))